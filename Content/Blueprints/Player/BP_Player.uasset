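; BP_Player is the player Blueprint, tracking Health and Money and handling game over.
; DamagePlayer subtracts health and, at zero or below, shows the WBP_GameOver widget with the mouse cursor, pauses the game and destroys the actor.
; AddMoney increases the money total.
; The K key calls DamagePlayer directly with a fixed amount, while BeginPlay, overlap and Tick events are unused.
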(event `Key|K`
  (params (Key :type "Key Structure"))
  (:`Pressed`
    (`self.DamagePlayer` 50)))

(fn `AddMoney`
  (params (Amount :type Integer))
  (set `self.Money` (+ (`self.Money`) Amount)))

(fn `DamagePlayer`
  (params (Amount :type Integer))
  (bind _returnvalue (`GameplayStatics.GetPlayerController` 0))
  (bind _output_get (set `self.Health` (- (`self.Health`) Amount)))
  ;[1 1 1] Player Health 0: game over logic
  (if (<= _output_get 0)
    (bind _returnvalue_2 (`|CreateWidget` "/Game/Blueprints/UI/WBP_GameOver.WBP_GameOver_C" _returnvalue))
    (`UserWidget.AddToViewport` _returnvalue_2 0)
    (set `PlayerController.bShowMouseCursor` true _returnvalue)
    (`GameplayStatics.SetGamePaused` true)
    (`self.K2_DestroyActor`)))

(fn `UserConstructionScript`)