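; BP_TestEnemy is a test enemy that travels along a spline path and can be killed by damage, including from turrets.
; On BeginPlay it finds the BP_EnemyPath actor and runs a timeline, rate-scaled by EnemyPathTime, that sets its transform along the spline.
; DamageEnemy reduces Health and, at zero, destroys the actor, decrements the player's RoundEnemyCount and awards money only for turret kills.
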(event `self.ReceiveBeginPlay`
  (bind _returnvalue (`GameplayStatics.GetActorOfClass` "/Game/Blueprints/Enemy/TestEnemy/BP_EnemyPath.BP_EnemyPath_C"))
  (set `self.EnemyPath` _returnvalue)
  (`self.FollowPath`))

(event `FollowPath`
  (bind _spline (`/Game/Blueprints/Enemy/TestEnemy/BP_EnemyPath.Spline` (`self.EnemyPath`)))
  (`TimelineComponent.SetPlayRate` (`self.FollowPathTimeline`) (/ 1.0 (`self.EnemyPathTime`)))
  (bind (_direction _followpath) (`Timeline|FollowPathTimeline`)
    (:`Update`
      (bind _returnvalue (`KismetMathLibrary.Lerp` 0.0 (`SplineComponent.GetSplineLength` (`/Game/Blueprints/Enemy/TestEnemy/BP_EnemyPath.Spline` (`self.EnemyPath`))) _followpath))
      (`self.K2_SetActorTransform` (`KismetMathLibrary.MakeTransform` (`SplineComponent.GetLocationAtDistanceAlongSpline` _spline _returnvalue "World") (`SplineComponent.GetRotationAtDistanceAlongSpline` _spline _returnvalue "Local"))))))

(fn `DamageEnemy`
  (params (Amount :type Integer) (FromTurret :type Boolean))
  (bind _output_get (set `self.Health` (- (`self.Health`) Amount)))
  (if (<= _output_get 0)
    (`self.K2_DestroyActor`)
    (bind _asbp_player (cast `/Game/Blueprints/Player/BP_Player` (`GameplayStatics.GetPlayerCharacter` 0)))
    (set `/Game/Blueprints/Player/BP_Player.Round Enemy Count` (- (`/Game/Blueprints/Player/BP_Player.Round Enemy Count` _asbp_player) 1) _asbp_player)
    (if FromTurret
      ;[1 1 1] Change amount of money given from each enemy
      (`/Game/Blueprints/Player/BP_Player.AddMoney` _asbp_player 20))))

(fn `UserConstructionScript`)