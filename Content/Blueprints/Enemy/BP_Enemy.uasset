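; Tower defense enemy that travels along the level's BP_EnemyPath spline and loses health to projectiles.
; FollowPath drives position and tangent-based rotation with a timeline, its play rate scaled by EnemyPathTime.
; Projectile overlaps destroy the projectile and call DamageEnemy, which updates the health bar or handles death.
; Death decrements the player's round enemy count, paying bounty only for turret kills; DestroyEnemy forces an unpaid death.
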(event `self.ReceiveBeginPlay`
  (bind _returnvalue (`GameplayStatics.GetActorOfClass` "/Game/Blueprints/Enemy/BP_EnemyPath.BP_EnemyPath_C"))
  (set `self.EnemyPath` _returnvalue))

(event `FollowPath`
  (bind _spline (`/Game/Blueprints/Enemy/BP_EnemyPath.Spline` (`self.EnemyPath`)))
  (`TimelineComponent.SetPlayRate` (`self.FollowPathTimeline`) (/ 1.0 (`self.EnemyPathTime`)))
  (bind (_direction _followpath) (`Timeline|FollowPathTimeline`)
    (:`Update`
      (bind _returnvalue (`KismetMathLibrary.Lerp` 0.0 (`SplineComponent.GetSplineLength` (`/Game/Blueprints/Enemy/BP_EnemyPath.Spline` (`self.EnemyPath`))) _followpath))
      (`self.K2_SetActorTransform` (`KismetMathLibrary.MakeTransform` (`SplineComponent.GetLocationAtDistanceAlongSpline` _spline _returnvalue "World") (`KismetMathLibrary.MakeRotationFromAxes` (`SplineComponent.GetTangentAtDistanceAlongSpline` _spline _returnvalue "Local")))))))

(event `self.SphereCollision.OnComponentBeginOverlap`
  (params (OverlappedComponent :type "PrimitiveComponent Object Reference") (OtherActor :type "Actor Object Reference") (OtherComp :type "PrimitiveComponent Object Reference") (OtherBodyIndex :type Integer) (bFromSweep :type Boolean) (SweepResult :type "HitResult Structure (by ref)"))
  (bind _asbp_projectile (cast `/Game/Blueprints/Projectile/BP_Projectile` OtherActor))
  (`self.K2_DestroyActor` _asbp_projectile)
  (`self.DamageEnemy` (`self.HealthDamage`) true))

(fn `DamageEnemy`
  (params (Amount :type Integer) (FromTurret :type Boolean))
  (bind _output_get (set `self.Health` (- (`self.Health`) Amount)))
  (if (<= _output_get 0)
    (`self.K2_DestroyActor`)
    (bind _asbp_player (cast `/Game/Blueprints/Player/BP_Player` (`GameplayStatics.GetPlayerCharacter` 0)))
    (set `/Game/Blueprints/Player/BP_Player.Round Enemy Count` (- (`/Game/Blueprints/Player/BP_Player.Round Enemy Count` _asbp_player) 1) _asbp_player)
    (if FromTurret
      ;[1 1 1] Change amount of money given from each enemy
      (`/Game/Blueprints/Player/BP_Player.AddMoney` _asbp_player (`self.Bounty`)))
    (else
      ;[1 1 1] Update enemy Health Bar
      (bind _aswbp_enemy_health (cast `/Game/Blueprints/Enemy/WBP_EnemyHealth` (`WidgetComponent.GetUserWidgetObject` (`self.HealthBar`))))
      (`/Game/Blueprints/Enemy/WBP_EnemyHealth.UpdateHealthbar` _aswbp_enemy_health (`KismetMathLibrary.Conv_IntToDouble` (/ (* (`self.Health`) 100) (`self.BaseHealth`)))))))

(fn `DestroyEnemy`
  (`self.DamageEnemy` 1000000000))

(fn `UserConstructionScript`)