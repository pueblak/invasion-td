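; Tower-defense grid cell that highlights on hover and, when clicked, buys the selected turret or opens the upgrade menu if occupied.
; Purchase deducts player money, applies that type's sprites, clears the shop selection and starts firing.
; A self-restarting RefireDelay timeline range-checks a cached enemy location before launching projectiles via SuggestProjectileVelocity.
; FireProjectile targets the last enemy from GetAllActorsOfClass; the nearest-enemy search is unfinished and never runs.
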(event `self.Collision.OnClicked`
  (params (TouchedComponent :type "PrimitiveComponent Object Reference") (ButtonPressed :type "Key Structure"))
  ;[1 1 1] Assign the selected cell to the turret type currently defined in the player controller
  (bind _astdcontroller (cast `/Game/Blueprints/Player/TDController` (`GameplayStatics.GetPlayerController` 0)))
  (if (`|EnumEquality` (`self.Type`) "NewEnumerator0")
    (bind _asbp_player (cast `/Game/Blueprints/Player/BP_Player` (`GameplayStatics.GetPlayerCharacter` 0)))
    (if (not (`|EnumEquality` (`/Game/Blueprints/Player/TDController.Purchased` _astdcontroller) "NewEnumerator0"))
      (bind _purchasecost (`/Game/Blueprints/Player/TDController.PurchaseCost` _astdcontroller))
      (if (>= (`/Game/Blueprints/Player/BP_Player.Money` _asbp_player) _purchasecost)
        (`/Game/Blueprints/Player/BP_Player.AddMoney` _asbp_player (* _purchasecost -1))
        (bind _purchased (`/Game/Blueprints/Player/TDController.Purchased` _astdcontroller))
        (if (`|EnumEquality` _purchased "NewEnumerator1")
          ;;[1 1 1] If more turret types are added in the future, then this structure is going to become incredibly difficult to handle. This should only be used as a placeholder
          (`self.PlaceTurretType1`)
          (set `/Game/Blueprints/Player/TDController.Purchased` "NewEnumerator0" _astdcontroller :!label _label) ; May want to get rid of this to allow player to add multiple turrets of the same type in quick succession
          (`/Game/Blueprints/UI/WBP_TurretShop.ClearSelection` (`/Game/Blueprints/Player/TDController.TurretShop` _astdcontroller))
          (`self.StartFiring`)
          (elif (`|EnumEquality` _purchased "NewEnumerator2")
            (`self.PlaceTurretType2`)
            (goto _label)
            (elif (`|EnumEquality` _purchased "NewEnumerator3")
              (`self.PlaceTurretType3`)
              (goto _label)
              (elif (`|EnumEquality` _purchased "NewEnumerator4")
                (`self.PlaceTurretType4`)
                (goto _label)))))))
    (else
      (`/Game/Blueprints/UI/WBP_HUD.Display Upgrade Menu` (`/Game/Blueprints/Player/TDController.HUD` _astdcontroller) self) ; So if a turret occupies this cell, open the upgrade menu
    )))

(event `self.Collision.OnBeginCursorOver`
  (params (TouchedComponent :type "PrimitiveComponent Object Reference"))
  ;[1 1 1] Highlight Hovered Cell
  (`SceneComponent.SetHiddenInGame` (`self.Collision`) false false))

(event `self.Collision.OnEndCursorOver`
  (params (TouchedComponent :type "PrimitiveComponent Object Reference"))
  ;[1 1 1] Highlight Hovered Cell
  (`SceneComponent.SetHiddenInGame` (`self.Collision`) true false))

(event `ContinueFiring`
  ;[1 1 1] Fire Projectile
  (if (== (`TimelineComponent.GetPlaybackPosition` (`self.TurretFire`)) 0.0) :!label _label_2
    (bind _outactors (`GameplayStatics.GetAllActorsOfClass` "/Game/Blueprints/Enemy/BP_Enemy.BP_Enemy_C"))
    (if (!= (`KismetArrayLibrary.Array_Length` _outactors) 0)
      (if (>= (`self.AttackRange`) (`KismetMathLibrary.VSize` (- (`self.ClosestActorLoc`) (`self.CurLocation`))))
        (`self.FireProjectile`)
        (`Timeline|TurretFire` :!label _label_3
          (:`Finished`
            (`self.ResetFireTimeline`)
            (`self.ContinueFiring`)))
        (else
          (goto _label_3)))
      (else
        (goto _label_3)))))

(event `StartFiring`
  ;[1 1 1] Fire Projectile
  (`TimelineComponent.SetTimelineLength` (`self.TurretFire`) (`self.RefireDelay`))
  (goto _label_2))

(event `ResetFireTimeline`
  ;[1 1 1] Fire Projectile
  (`|ExecutionSequence`
    (:`then_0`
      (goto _label_3 :!via `Stop`))
    (:`then_1`
      (goto _label_3 :!via `SetNewTime`))))

(event `FireProjectile`
  (bind _returnvalue (+ (`self.K2_GetActorLocation`) (* (`self.GetActorForwardVector`) 10.0) (0.0 5.0 0.0)))
  ;[1 1 1] Fire Projectile
  (set `self.CurLocation` (`SceneComponent.GetSocketLocation` (`self.BaseSprite`) "None"))
  (bind _outactors (`GameplayStatics.GetAllActorsOfClass` "/Game/Blueprints/Enemy/BP_Enemy.BP_Enemy_C"))
  (set `self.ClosestActorLoc` (`self.K2_GetActorLocation` (`|GetArrayItem` _outactors (- (`KismetArrayLibrary.Array_Length` _outactors) 1))))
  (bind _returnvalue_2 (`|SpawnActorFromClass` "/Game/Blueprints/Projectile/BP_Projectile.BP_Projectile_C" (`KismetMathLibrary.MakeTransform` _returnvalue (struct) (0.25 0.25 0.25)) "Undefined" "OverrideRootScale" null null))
  (bind _tossvelocity (`GameplayStatics.BlueprintSuggestProjectileVelocity` _returnvalue (`self.ClosestActorLoc`) 1000.0 0.0 "DoNotTrace"))
  (`ProjectileMovementComponent.SetVelocityInLocalSpace` (`/Game/Blueprints/Projectile/BP_Projectile.ProjectileMovement` _returnvalue_2) _tossvelocity))

(fn `PlaceTurretType1`
  (`PaperSpriteComponent.SetSprite` (`self.BaseSprite`) "/Game/Sprites/Turret/turret4/turret4_base1_Sprite.turret4_base1_Sprite")
  (`PaperSpriteComponent.SetSprite` (`self.PrimarySprite`) "/Game/Sprites/Turret/turret4/turret4_primary1_Sprite.turret4_primary1_Sprite")
  (set `self.Type` "NewEnumerator1"))

(fn `PlaceTurretType2`
  (`PaperSpriteComponent.SetSprite` (`self.BaseSprite`) "/Game/Sprites/Turret/turret3/turret3_base1_Sprite.turret3_base1_Sprite")
  (`PaperSpriteComponent.SetSprite` (`self.PrimarySprite`) "/Game/Sprites/Turret/turret3/turret3_primary1_Sprite.turret3_primary1_Sprite")
  (set `self.Type` "NewEnumerator2"))

(fn `PlaceTurretType3`
  (`PaperSpriteComponent.SetSprite` (`self.BaseSprite`) "/Game/Sprites/Turret/turret2/turret2_base1_Sprite.turret2_base1_Sprite")
  (`PaperSpriteComponent.SetSprite` (`self.PrimarySprite`) "/Game/Sprites/Turret/turret2/turret2_primary1_Sprite.turret2_primary1_Sprite")
  (set `self.Type` "NewEnumerator3"))

(fn `PlaceTurretType4`
  (`PaperSpriteComponent.SetSprite` (`self.BaseSprite`) "/Game/Sprites/Turret/turret1/turret1_base1_Sprite.turret1_base1_Sprite")
  (`PaperSpriteComponent.SetSprite` (`self.PrimarySprite`) "/Game/Sprites/Turret/turret1/turret1_primary1_Sprite.turret1_primary1_Sprite")
  (set `self.Type` "NewEnumerator4"))

(fn `UserConstructionScript`)